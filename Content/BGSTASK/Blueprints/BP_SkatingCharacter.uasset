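; Skating character Blueprint that turns the IA_SkateMove input into push, brake and steer movement.
; Positive Y adds half-scale forward input; zero or negative Y brakes forward motion by lerping horizontal velocity toward zero on each trigger.
; X adds half-scale sideways input only while pushing or already moving.
; GetMovementInput returns both input axes and velocity, printing them for debugging.
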(event Input|EnhancedActionEvents|EnhancedInputActionIA_SkateMove
  (params (ActionValue :type Vector%202D%20Structure) (ElapsedSeconds :type Float%20%28double-precision%29) (TriggeredSeconds :type Float%20%28double-precision%29) (InputAction :type Input%20Action%20Object%20Reference :default "/Game/BGSTASK/Inputs/IA_SkateMove.IA_SkateMove"))
  (bind _returnvalue (Transformation|GetVelocity))
  (bind (_x _y) (Math|Vector2D|BreakVector2D ActionValue))
  (bind _charactermovement (Variables|Character|GetCharacterMovement))
  (bind _returnvalue_2 (> _y 0.0))
  (:Triggered
    (Utilities|FlowControl|Sequence
      (:then_0
        (if _returnvalue_2
          (Pawn|Input|AddMovementInput (Transformation|GetActorForwardVector) (* _y 0.5) false)
          (elif (> (.x (Math|Vector|UnrotateVector _returnvalue (Transformation|GetActorRotation))) 0.0)
            (Variables|/Script/Engine.MovementComponent|SetVelocity _charactermovement (Math|Vector|MakeVector (Math|Float|Lerp (.x (Variables|/Script/Engine.MovementComponent|GetVelocity _charactermovement)) 0.0 0.1) (Math|Float|Lerp (.y (Variables|/Script/Engine.MovementComponent|GetVelocity _charactermovement)) 0.0 0.1) (.z (Variables|/Script/Engine.MovementComponent|GetVelocity _charactermovement)))))))
      (:then_1
        (if (or _returnvalue_2 (> (Math|Vector|VectorLength _returnvalue) 5.0))
          (Pawn|Input|AddMovementInput (Transformation|GetActorRightVector) (* _x 0.5) false))))))

(fn ConstructionScript
  (|CallParentFunction))

(fn GetMovementInput
  (bind _returnvalue (Transformation|GetVelocity))
  (bind _returnvalue_2 (Input|EnhancedActionValues|GetIA_SkateMove))
  (bind (_x _y) (Math|Vector2D|BreakVector2D _returnvalue_2))
  (Development|PrintString (Utilities|String|Append (Utilities|String|ToString(Vector2d) _returnvalue_2) " -- " (Utilities|String|ToString(Vector) _returnvalue)) true true "(R=0.000000,G=0.660000,B=1.000000,A=1.000000)" 0.0)
  (return _y _x _returnvalue))