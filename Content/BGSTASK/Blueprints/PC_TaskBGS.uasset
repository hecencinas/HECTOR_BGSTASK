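; Player controller for a skating game that awards points for obstacles jumped over and creates the main UI widget.
; It binds to the skating character's jump-start and landed events, saving the takeoff position.
; On landing, a multi-object capsule trace between offset takeoff and landing points ignores the skater and landed-on actor, adds the hit count to Points and broadcasts the update.
; An optional debug draw visualizes the trace and hits.
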(event Custom|LandedDelegate_Event
  (params (Hit :type Hit%20Result%20Structure%20%28by%20ref%29))
  (bind (_bblockinghit _binitialoverlap _time _distance _location _impactpoint _normal _impactnormal _physmat _hitactor) (Collision|BreakHitResult Hit))
  (bind _offset (Variables|Default|GetOffset))
  (bind _offset_2 (Variables|Default|GetOffset))
  (bind _positiononjumpstart (Variables|Default|GetPositionOnJumpStart))
  (bind _returnvalue (+ _location _offset))
  (bind _returnvalue_2 (+ _positiononjumpstart _offset_2))
  (if (Variables|Default|GetJumping)
    (Variables|Default|SetJumping false)
    (Utilities|FlowControl|Sequence
      (:then_0
        (bind _outhits (Class|KismetSystemLibrary|CapsuleTraceMultiforObjects _returnvalue_2 _returnvalue (Variables|Default|GetObstacleDetectionRadius) 0.0 (Utilities|Array|MakeArray "ObjectTypeQuery1" "ObjectTypeQuery2" "ObjectTypeQuery6" "ObjectTypeQuery3") false (Utilities|Array|MakeArray (Variables|Default|GetSkatingCharacter) _hitactor) "None" true))
        (bind _output_get (Variables|Default|SetPoints (+ (Utilities|Array|Length _outhits) (Variables|Default|GetPoints))))
        (Default|CallPointsUpdate _output_get))
      (:then_1
        (CallFunction|DebugJumpOverObstacle _outhits _returnvalue_2 _returnvalue (Variables|Default|GetDebugDuration) (Variables|Default|GetObstacleDetectionRadius))))))

(event Custom|OnCharacterJumpStart_Event
  (Variables|Default|SetPositionOnJumpStart (Transformation|GetActorLocation (Variables|Default|GetSkatingCharacter)))
  (Variables|Default|SetJumping true))

(event EventBeginPlay
  (Utilities|FlowControl|Sequence
    (:then_0
      (bind _asbp_skating_character (Utilities|Casting|CastToBP_SkatingCharacter (Pawn|GetControlledPawn)))
      (bind _output_get (Variables|Default|SetSkatingCharacter _asbp_skating_character))
      (EventDispatchers|AssignLandedDelegate _output_get (EventDispatchers|CreateEvent :!event Custom|LandedDelegate_Event))
      (EventDispatchers|BindEventtoOnJumpStart (Variables|Default|GetSkatingCharacter) (EventDispatchers|CreateEvent :!event Custom|OnCharacterJumpStart_Event)))
    (:then_1
      (bind _returnvalue (UserInterface|CreateWidget "/Game/BGSTASK/Widgets/WBP_GameMainUI.WBP_GameMainUI_C" self))
      (bind _output_get_2 (Variables|Default|SetMainUI _returnvalue))
      (UserInterface|Viewport|AddtoViewport _output_get_2 0))))

(fn ConstructionScript)

(fn DebugJumpOverObstacle
  (params (Hits :type Array%20of%20Hit%20Result%20Structures) (Start :type Vector) (End :type Vector%20%28by%20ref%29) (Duration :type Float%20%28single-precision%29) (Radius :type Float%20%28double-precision%29))
  (bind _returnvalue (Math|Vector|MakeVector Radius 0.0 0.0))
  (bind _returnvalue_2 (Math|Vector|MakeVector Radius 0.0 0.0))
  (bind _returnvalue_3 (Math|Vector|MakeVector 0.0 0.0 Radius))
  (bind _returnvalue_4 (Math|Vector|MakeVector 0.0 0.0 Radius))
  (if (Variables|Default|GetDebugEnabled)
    (Utilities|FlowControl|Sequence
      (:then_0
        ;[1 1 1] debug trace start/end points
        (Rendering|Debug|DrawDebugSphere Start Radius 12 "(R=1.000000,G=0.000000,B=0.000000,A=1.000000)" Duration)
        (Rendering|Debug|DrawDebugSphere End Radius 12 "(R=1.000000,G=0.000000,B=0.000000,A=1.000000)" Duration))
      (:then_1
        ;[1 1 1] debug lines for capsule visualization
        (Rendering|Debug|DrawDebugLine Start End "(R=0.000000,G=0.000000,B=1.000000,A=1.000000)" Duration 0.0)
        (Rendering|Debug|DrawDebugLine (+ Start _returnvalue_3) (+ End _returnvalue_3) "(R=0.000000,G=0.000000,B=1.000000,A=1.000000)" Duration 0.0)
        (Rendering|Debug|DrawDebugLine (- Start _returnvalue_4) (- End _returnvalue_4) "(R=0.000000,G=0.000000,B=1.000000,A=1.000000)" Duration 0.0)
        (Rendering|Debug|DrawDebugLine (+ Start _returnvalue) (+ End _returnvalue) "(R=0.000000,G=0.000000,B=1.000000,A=1.000000)" Duration 0.0)
        (Rendering|Debug|DrawDebugLine (- Start _returnvalue_2) (- End _returnvalue_2) "(R=0.000000,G=0.000000,B=1.000000,A=1.000000)" Duration 0.0))
      (:then_2
        ;[1 1 1] debug hit points
        (for _array_element Hits
          (Rendering|Debug|DrawDebugSphere (.ImpactPoint (Collision|BreakHitResult _array_element)) Radius 12 "(R=0.000000,G=1.000000,B=0.000000,A=1.000000)" Duration))))))